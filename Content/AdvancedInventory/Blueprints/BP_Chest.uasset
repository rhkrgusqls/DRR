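; Inventory chest that fills itself with randomized starting loot on BeginPlay and holds its slot items and visibility flags.
; Slot count comes from a temporary WB_ChestUI, counting children of its horizontal bars, so the UI layout sets capacity.
; Each starting item rolls chance and amount, loads its Item_Table row by ID, and lands in an optionally shuffled slot.
; UpdateChestSlots stores changed slots and has BP_InventoryGameMode update players within the chest's radius.
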(event Custom|UpdateChestSlots
  (params (visibilities :type Array%20of%20Booleans) (items :type Array%20of%20Item%20Structur%20Structures) (PC :type Player%20Controller%20Object%20Reference))
  ;[1 1 1] Update the slots of the chest on server
  (Variables|Default|SetVisibility_items visibilities)
  (Variables|Default|SetData_items items)
  (Default|UpdateChestforPlayersWhoAreinRadiusOftheChest (CallFunction|GetGM) self PC visibilities items))

(event Custom|SetUpChestItems
  ;[1 1 1] Add chest items on EventBeginPlay
  (if (Variables|Default|GetRandomSorting?)
    (Utilities|Array|Shuffle (Variables|Default|GetShuffle)))
  (for (_array_element _array_index) (Variables|Default|GetStartingItems)
    (bind _output_get (Variables|Default|SetPercentageValue (Math|Random|RandomIntegerinRange 0 100)))
    (if (>= (.ProbabilityToAppear_0to100 (Utilities|Struct|BreakAddItemIDandAmount_Structure _array_element)) _output_get)
      (Variables|Default|SetAmount (Math|Random|RandomIntegerinRange (.AmountMinimum (Utilities|Struct|BreakAddItemIDandAmount_Structure _array_element)) (.AmountMaximum (Utilities|Struct|BreakAddItemIDandAmount_Structure _array_element))))
      (bind _returnvalue (Utilities|GetDataTableRow "/Game/AdvancedInventory/Item_Table.Item_Table" (select (== (.ID (Utilities|Struct|BreakAddItemIDandAmount_Structure _array_element)) 0) (Utilities|Name|MakeLiteralName "NewRow") (Utilities|String|StringToName (Utilities|String|Append "NewRow_" (Utilities|String|ToString(Integer) (- (.ID (Utilities|Struct|BreakAddItemIDandAmount_Structure _array_element)) 1))))))
        (:then
          (bind _structout (Utilities|Struct|SetmembersinItem_Structur _returnvalue (Math|Integer|SelectInt (Math|Integer|SelectInt (.maximumStackSize (Utilities|Struct|BreakItem_Structur _returnvalue)) (Variables|Default|GetAmount) (> (Variables|Default|GetAmount) (.maximumStackSize (Utilities|Struct|BreakItem_Structur _returnvalue)))) 1 (.Stackable (Utilities|Struct|BreakItem_Structur _returnvalue)))))
          (Utilities|Array|SetArrayElem (Variables|Default|GetData_items) (Utilities|Array|Get(acopy) (Variables|Default|GetShuffle) _array_index) _structout)
          (Utilities|Array|SetArrayElem (Variables|Default|GetVisibility_items) (Utilities|Array|Get(acopy) (Variables|Default|GetShuffle) _array_index) true))))))

(event EventBeginPlay
  ;[1 1 1] Add chest items on EventBeginPlay
  (bind _newparam (CallFunction|CountChestSlots))
  (for _index (range 0 (- _newparam 1))
    (Utilities|Array|Add (Variables|Default|GetVisibility_items) false)
    (Utilities|Array|Add :TargetArray (Variables|Default|GetData_items))
    (Utilities|Array|Add (Variables|Default|GetShuffle) _index))
  (CallFunction|SetUpChestItems))

(fn ConstructionScript)

(fn CountChestSlots
  ;[1 1 1] Get the amount of the chest slots from the UI -> So you can add a certain amount of chest slots in your ChestUI
  (bind _returnvalue (UserInterface|CreateWidget "/Game/Asset/UI/Inventory/WB_ChestUI.WB_ChestUI_C"))
  (for _array_element (Class|PanelWidget|GetAllChildren (Variables|/Game/Asset/UI/Inventory/WB_ChestUI.WB_ChestUI_C|GetChestBars _returnvalue))
    (bind _ashorizontal_box (Utilities|Casting|CastToHorizontalBox _array_element))
    (LocalVariables|SetcountVar (+ (LocalVariables|GetcountVar) (Class|PanelWidget|GetChildrenCount _ashorizontal_box))))
  (return (LocalVariables|GetcountVar)))

(fn GetGM
  (bind _asbp_inventory_game_mode (Utilities|Casting|CastToBP_InventoryGameMode (Game|GetGameMode)))
  (return _asbp_inventory_game_mode))