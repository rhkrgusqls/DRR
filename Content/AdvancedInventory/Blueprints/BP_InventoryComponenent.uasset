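; Inventory component that handles the player's world interaction: dropping items, picking them up, chest proximity and the nearby ground-item list.
; A looping camera line trace focuses drop actors and toggles pickup info, feeding manual Pickup, while overlaps drive optional auto-pickup.
; Items are added through BP_InventoryPlayerController, and drops spawn at the player with camera pitch setting vertical velocity.
; Overlap events show or hide chest UI and rebuild ground-list widgets through the HUD.
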(event Custom|Reset
  ;[1 1 1] Looping timer for focusing an item
  (Utilities|FlowControl|DoOnce false) ; enters at Reset
)

(event Custom|Pickup
  ;[1 1 1] Pick up a focused item
  (if (Variables|Default|GetisFocusingItem?)
    (Utilities|IsValid (Variables|Default|GetFocusedItem)
      (:Is%20Valid
        (bind _asbp_drop_item_actor_master (Utilities|Casting|CastToBP_DropItemActor_Master (Variables|Default|GetFocusedItem)))
        (Default|AddItem (CallFunction|GetPC) (.ID (Utilities|Struct|BreakItem_Structur (Variables|/Game/AdvancedInventory/Blueprints/BP_DropItemActor_Master.BP_DropItemActor_Master_C|GetItemData _asbp_drop_item_actor_master))) (.amount (Utilities|Struct|BreakItem_Structur (Variables|/Game/AdvancedInventory/Blueprints/BP_DropItemActor_Master.BP_DropItemActor_Master_C|GetItemData _asbp_drop_item_actor_master))))
        (Default|DestroyActorfromPC (CallFunction|GetPC) (Variables|Default|GetFocusedItem))
        (CallFunction|Reset)))))

(event Custom|LinetraceLoop
  (bind _returnvalue (Game|GetPlayerCameraManager 0))
  (bind _returnvalue_2 (Camera|GetCameraLocation _returnvalue))
  ;[1 1 1] Looping timer for focusing an item
  (bind (_outhit _returnvalue_3) (Collision|LineTraceByChannel _returnvalue_2 (+ _returnvalue_2 (* (Math|Vector|GetForwardVector (Camera|GetCameraRotation _returnvalue)) 8e+02)) "TraceTypeQuery1" false 0 "None"))
  (if _returnvalue_3
    (if (== (Utilities|GetClass (.HitActor (Collision|BreakHitResult _outhit))) "/Game/AdvancedInventory/Blueprints/BP_DropItemActor_Master.BP_DropItemActor_Master_C")
      (Utilities|FlowControl|Sequence
        (:then_0
          (bind _asbp_drop_item_actor_master (Utilities|Casting|CastToBP_DropItemActor_Master (.HitActor (Collision|BreakHitResult _outhit))))
          (if (Math|Boolean|ORBoolean (!= (.ID (Utilities|Struct|BreakItem_Structur (Variables|/Game/AdvancedInventory/Blueprints/BP_DropItemActor_Master.BP_DropItemActor_Master_C|GetItemData _asbp_drop_item_actor_master))) (Variables|Default|GetcompareID)) (!= (.amount (Utilities|Struct|BreakItem_Structur (Variables|/Game/AdvancedInventory/Blueprints/BP_DropItemActor_Master.BP_DropItemActor_Master_C|GetItemData _asbp_drop_item_actor_master))) (Variables|Default|GetcompareAmount)) (!= (.HitActor (Collision|BreakHitResult _outhit)) (Variables|Default|GetFocusedItem)))
            (Variables|Default|SetcompareID (.ID (Utilities|Struct|BreakItem_Structur (Variables|/Game/AdvancedInventory/Blueprints/BP_DropItemActor_Master.BP_DropItemActor_Master_C|GetItemData _asbp_drop_item_actor_master))))
            (Variables|Default|SetcompareAmount (.amount (Utilities|Struct|BreakItem_Structur (Variables|/Game/AdvancedInventory/Blueprints/BP_DropItemActor_Master.BP_DropItemActor_Master_C|GetItemData _asbp_drop_item_actor_master))))
            (bind _asbp_my_hud (Utilities|Casting|CastToBP_MyHUD (HUD|GetHUD (Game|GetPlayerController 0))))
            (Default|ShowPickUpInfo (Variables|/Game/AdvancedInventory/Widgets/WB_UI.WB_UI_C|GetInventory (Variables|/Game/AdvancedInventory/Blueprints/BP_MyHUD.BP_MyHUD_C|GetUI_Ref _asbp_my_hud)) true (Variables|/Game/AdvancedInventory/Blueprints/BP_DropItemActor_Master.BP_DropItemActor_Master_C|GetItemData _asbp_drop_item_actor_master))
            (Variables|Default|SetFocusedItem (.HitActor (Collision|BreakHitResult _outhit)))
            (if (not (Variables|Default|GetisFocusingItem?))
              (Variables|Default|SetisFocusingItem? true))))
        (:then_1
          (goto _label Reset)))
      (else
        (Utilities|FlowControl|DoOnce false :!label _label
          (:Completed
            (Variables|Default|SetcompareAmount -1)
            (Variables|Default|SetcompareID -1)
            (bind _asbp_my_hud_2 (Utilities|Casting|CastToBP_MyHUD (HUD|GetHUD (Game|GetPlayerController 0))))
            (Default|ShowPickUpInfo (Variables|/Game/AdvancedInventory/Widgets/WB_UI.WB_UI_C|GetInventory (Variables|/Game/AdvancedInventory/Blueprints/BP_MyHUD.BP_MyHUD_C|GetUI_Ref _asbp_my_hud_2)) false)
            (Variables|Default|SetisFocusingItem? false)))))
    (else
      (goto _label))))

(event Custom|On%28End%29Overlap%20ItemRadiusForGroundList
  ;[1 1 1] Update the GroundItemList when the radius overlaps or ends to overlap an item
  (CallFunction|UpdateGroundItemList))

(event Custom|SpawnItemOnServer
  (params (SpawnTransform :type Transform) (Speed :type Float%20%28double-precision%29) (ItemData :type Item%20Structur%20Structure) (zVelocity :type Float%20%28double-precision%29) (xVelocity :type Float%20%28double-precision%29))
  ;[1 1 1] Drop an item
  (Game|SpawnActorfromClass "/Game/AdvancedInventory/Blueprints/BP_DropItemActor_Master.BP_DropItemActor_Master_C" SpawnTransform "Undefined" "OverrideRootScale" 0 Speed ItemData zVelocity xVelocity 0))

(event Custom|DropEvent
  (params (ItemData :type Item%20Structur%20Structure))
  (bind _returnvalue (Game|GetPlayerCharacter 0))
  (bind _returnvalue_2 (Transformation|GetActorLocation _returnvalue))
  (bind (_x _y _z) (Math|Vector|BreakVector _returnvalue_2))
  ;[1 1 1] Drop an item
  (CallFunction|SpawnItemonServer (Math|Transform|MakeTransform (Math|Vector|MakeVector _x _y (+ 4e+01 _z)) (Math|Rotator|MakeRotator 0.0 0.0 (.Yaw (Math|Rotator|BreakRotator (Transformation|GetActorRotation _returnvalue))))) (Variables|Default|GetRandomItemDropSpeed) ItemData (* (.Pitch (Math|Rotator|BreakRotator (Camera|GetCameraRotation (Game|GetPlayerCameraManager 0)))) 12.0) 0.0))

(event Custom|ActorEndOverlap
  (params (Actor :type Actor%20Object%20Reference))
  ;[1 1 1] Hide the chestUI when the player leaves the radius of a chest
  (if (== (Utilities|GetClass Actor) "/Game/AdvancedInventory/Blueprints/BP_Chest.BP_Chest_C")
    (Variables|Default|SetisOverlapping%20Chest? false)
    (bind _asbp_my_hud (Utilities|Casting|CastToBP_MyHUD (HUD|GetHUD (Game|GetPlayerController 0))))
    (Default|Hide (Variables|/Game/AdvancedInventory/Widgets/WB_Inventory.WB_Inventory_C|GetChestUI (Variables|/Game/AdvancedInventory/Widgets/WB_UI.WB_UI_C|GetInventory (Variables|/Game/AdvancedInventory/Blueprints/BP_MyHUD.BP_MyHUD_C|GetUI_Ref _asbp_my_hud))))))

(event Custom|Setup
  ;[1 1 1] SetUp
  (Variables|/Game/AdvancedInventory/Blueprints/BP_InventoryPlayerController.BP_InventoryPlayerController_C|SetInventoryComponentRef (CallFunction|GetPC) self))

(event Custom|StartLineTraceLoop
  ;[1 1 1] Looping timer for focusing an item
  (Utilities|Time|SetTimerbyEvent (delegate Custom|LinetraceLoop) 0.15 true))

(event Custom|PickUpAllItemsBeginOverlap
  (params (Actor :type Actor%20Object%20Reference))
  ;[1 1 1] Auto Pickup Mode - The player automatically picks up an item when the character collides with it
  (if (Variables|/Game/AdvancedInventory/Blueprints/BP_InventoryPlayerController.BP_InventoryPlayerController_C|GetAutoPickupItemsMode (CallFunction|GetPC))
    (if (== (Utilities|GetClass Actor) "/Game/AdvancedInventory/Blueprints/BP_DropItemActor_Master.BP_DropItemActor_Master_C")
      (bind _asbp_drop_item_actor_master (Utilities|Casting|CastToBP_DropItemActor_Master Actor))
      (Default|AddItem (CallFunction|GetPC) (.ID (Utilities|Struct|BreakItem_Structur (Variables|/Game/AdvancedInventory/Blueprints/BP_DropItemActor_Master.BP_DropItemActor_Master_C|GetItemData _asbp_drop_item_actor_master))) (.amount (Utilities|Struct|BreakItem_Structur (Variables|/Game/AdvancedInventory/Blueprints/BP_DropItemActor_Master.BP_DropItemActor_Master_C|GetItemData _asbp_drop_item_actor_master))))
      (Default|DestroyActorfromPC (CallFunction|GetPC) _asbp_drop_item_actor_master)
      (CallFunction|Reset))))

(event Custom|Reactivate
  ;[1 1 1] Auto Pickup Mode - The player automatically picks up an item when the character collides with it
  (if (Variables|/Game/AdvancedInventory/Blueprints/BP_InventoryPlayerController.BP_InventoryPlayerController_C|GetAutoPickupItemsMode (CallFunction|GetPC))
    (if (== (Utilities|GetClass (stale Custom|PickUpAllItemsBeginOverlap Actor)) "/Game/AdvancedInventory/Blueprints/BP_DropItemActor_Master.BP_DropItemActor_Master_C")
      (bind _asbp_drop_item_actor_master (Utilities|Casting|CastToBP_DropItemActor_Master (stale Custom|PickUpAllItemsBeginOverlap Actor)))
      (Default|AddItem (CallFunction|GetPC) (.ID (Utilities|Struct|BreakItem_Structur (Variables|/Game/AdvancedInventory/Blueprints/BP_DropItemActor_Master.BP_DropItemActor_Master_C|GetItemData _asbp_drop_item_actor_master))) (.amount (Utilities|Struct|BreakItem_Structur (Variables|/Game/AdvancedInventory/Blueprints/BP_DropItemActor_Master.BP_DropItemActor_Master_C|GetItemData _asbp_drop_item_actor_master))))
      (Default|DestroyActorfromPC (CallFunction|GetPC) _asbp_drop_item_actor_master)
      (CallFunction|Reset))))

(event Custom|ActorBeginOverlap
  (params (Actor :type Actor%20Object%20Reference))
  ;[1 1 1] Show the chestUI when the player enters the radius of a chest
  (if (== (Utilities|GetClass Actor) "/Game/AdvancedInventory/Blueprints/BP_Chest.BP_Chest_C")
    (Variables|Default|SetisOverlapping%20Chest? true)
    (bind _asbp_chest (Utilities|Casting|CastToBP_Chest Actor))
    (bind _asbp_my_hud (Utilities|Casting|CastToBP_MyHUD (HUD|GetHUD (Game|GetPlayerController 0))))
    (Default|UpateOwnChestUI (Variables|/Game/AdvancedInventory/Widgets/WB_Inventory.WB_Inventory_C|GetChestUI (Variables|/Game/AdvancedInventory/Widgets/WB_UI.WB_UI_C|GetInventory (Variables|/Game/AdvancedInventory/Blueprints/BP_MyHUD.BP_MyHUD_C|GetUI_Ref _asbp_my_hud))) _asbp_chest (Variables|/Game/AdvancedInventory/Blueprints/BP_Chest.BP_Chest_C|GetVisibility_items _asbp_chest) (Variables|/Game/AdvancedInventory/Blueprints/BP_Chest.BP_Chest_C|GetData_items _asbp_chest))
    (Default|Show (Variables|/Game/AdvancedInventory/Widgets/WB_Inventory.WB_Inventory_C|GetChestUI (Variables|/Game/AdvancedInventory/Widgets/WB_UI.WB_UI_C|GetInventory (Variables|/Game/AdvancedInventory/Blueprints/BP_MyHUD.BP_MyHUD_C|GetUI_Ref _asbp_my_hud))))))

(event EventBeginPlay
  ;[1 1 1] Looping timer for focusing an item
  (CallFunction|StartLineTraceLoop))

(fn UpdateGroundItemList
  (bind _pc (CallFunction|GetPC))
  (bind _groundradiusref (Variables|/Game/AdvancedInventory/Blueprints/BP_InventoryPlayerController.BP_InventoryPlayerController_C|GetGroundRadiusRef _pc))
  ;[1 1 1] Update GroundItemList - Clear all children from the list, get all items of the "ItemRadiusForGroundList"-Component and add the new GroundItem children
  (bind _asbp_my_hud (Utilities|Casting|CastToBP_MyHUD (HUD|GetHUD (Game|GetPlayerController 0))))
  (Utilities|IsValid (Variables|/Game/AdvancedInventory/Blueprints/BP_MyHUD.BP_MyHUD_C|GetUI_Ref _asbp_my_hud)
    (:Is%20Valid
      (Widget|Panel|ClearChildren (Variables|/Game/AdvancedInventory/Widgets/WB_GroundItems.WB_GroundItems_C|Getitems (Variables|/Game/AdvancedInventory/Widgets/WB_Inventory.WB_Inventory_C|GetGroundItems (Variables|/Game/AdvancedInventory/Widgets/WB_UI.WB_UI_C|GetInventory (Variables|/Game/AdvancedInventory/Blueprints/BP_MyHUD.BP_MyHUD_C|GetUI_Ref _asbp_my_hud)))))
      (Utilities|IsValid _groundradiusref
        (:Is%20Valid
          (for _array_element (Collision|GetOverlappingActors _groundradiusref "/Game/AdvancedInventory/Blueprints/BP_DropItemActor_Master.BP_DropItemActor_Master_C" :!class /Script/Engine.PrimitiveComponent)
            (bind _asbp_drop_item_actor_master (Utilities|Casting|CastToBP_DropItemActor_Master _array_element))
            (bind _returnvalue (UserInterface|CreateWidget "/Game/AdvancedInventory/Widgets/WB_GroundWidget.WB_GroundWidget_C" 0 (.image (Utilities|Struct|BreakItem_Structur (Variables|/Game/AdvancedInventory/Blueprints/BP_DropItemActor_Master.BP_DropItemActor_Master_C|GetItemData _asbp_drop_item_actor_master))) (Variables|/Game/AdvancedInventory/Widgets/WB_UI.WB_UI_C|GetInventory (Variables|/Game/AdvancedInventory/Blueprints/BP_MyHUD.BP_MyHUD_C|GetUI_Ref _asbp_my_hud))))
            (Widget|Panel|AddChild (Variables|/Game/AdvancedInventory/Widgets/WB_GroundItems.WB_GroundItems_C|Getitems (Variables|/Game/AdvancedInventory/Widgets/WB_Inventory.WB_Inventory_C|GetGroundItems (Variables|/Game/AdvancedInventory/Widgets/WB_UI.WB_UI_C|GetInventory (Variables|/Game/AdvancedInventory/Blueprints/BP_MyHUD.BP_MyHUD_C|GetUI_Ref _asbp_my_hud)))) _returnvalue)
            (Default|SetuporUpdate _returnvalue (.amount (Utilities|Struct|BreakItem_Structur (Variables|/Game/AdvancedInventory/Blueprints/BP_DropItemActor_Master.BP_DropItemActor_Master_C|GetItemData _asbp_drop_item_actor_master))) _array_element)))))))

(fn GetPC
  (bind _asbp_inventory_player_controller (Utilities|Casting|CastToBP_InventoryPlayerController (Game|GetPlayerController 0)))
  (return _asbp_inventory_player_controller))