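; Player controller for an inventory system, handling hotbar selection, inventory toggling, right-click equipping, auto-pickup and debug item-adding keys.
; It drives widgets through BP_MyHUD and sends equip messages to the player character; wheel and middle click just toggle the first two slots.
; Chest, item-amount and destroy requests go to BP_InventoryGameMode, while drops and ground lists go to the inventory component.
; Save/load flattens inventory and equipment slots into SaveGame arrays.
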(event Custom|Add%20Item
  (params (ID :type Integer) (Amount :type Integer))
  ;[1 0.1453 0.1354 1 142] Add this to your Playercontroller
  ;;[1 1 1] Add an item, amount can be bigger than maximum stack size
  (bind _asbp_my_hud (Utilities|Casting|CastToBP_MyHUD (HUD|GetHUD)))
  (Default|AddItem (Variables|/Game/Asset/UI/Inventory/WB_UI.WB_UI_C|GetInventory (Variables|/Game/AdvancedInventory/Blueprints/BP_MyHUD.BP_MyHUD_C|GetUI_Ref _asbp_my_hud)) ID Amount))

(event Custom|UpdateChestPC
  (params (Chest :type Object%20Object%20Reference) (visibilities :type Array%20of%20Booleans) (items :type Array%20of%20Item%20Structur%20Structures) (PC :type Player%20Controller%20Object%20Reference))
  ;[1 0.1453 0.1354 1 142] Add this to your Playercontroller
  ;;[1 1 1] Call the GameMode for an update of a specific chest
  (Default|UpdateChestGM (CallFunction|GetGM) Chest visibilities items PC))

(event Custom|UpdateItem
  (params (amount :type Integer) (NewParam :type Actor%20Object%20Reference))
  ;[1 0.1453 0.1354 1 142] Add this to your Playercontroller
  ;;[1 1 1 1 30] For the GroundItemList
  ;;;[1 1 1] Update the amount of an item
  (Default|UpdateAmountOfASpecificItem (CallFunction|GetGM) NewParam amount))

(event Custom|SelectTheNewSlotSlot
  ;[1 0.1453 0.1354 1 142] Add this to your Playercontroller
  ;;[1 1 1 1 30] selection event for mouse wheel and keyboard input
  (bind _asbp_my_hud (Utilities|Casting|CastToBP_MyHUD (HUD|GetHUD)))
  (bind _aswb_slot (Utilities|Casting|CastToWB_Slot (Class|PanelWidget|GetChildat (Variables|/Game/Asset/UI/Inventory/WB_Inventory.WB_Inventory_C|GetHotbar (Variables|/Game/Asset/UI/Inventory/WB_UI.WB_UI_C|GetInventory (Variables|/Game/AdvancedInventory/Blueprints/BP_MyHUD.BP_MyHUD_C|GetUI_Ref _asbp_my_hud))) (Variables|Default|GetcurrentSlot))))
  (Default|Select _aswb_slot true)
  (CallFunction|GetNewSlotDataandCallUpdateforCharcater))

(event Custom|DestroyActorFromPC
  (params (TargetActor :type Actor%20Object%20Reference))
  ;[1 0.1453 0.1354 1 142] Add this to your Playercontroller
  ;;[1 1 1] Destroy an actor replicated
  (Default|DestroyActorfromGM (CallFunction|GetGM) TargetActor))

(event Custom|UpdateWhenThsPCisInRadiusOfTheChest
  (params (chest :type BP%20Chest%20Object%20Reference) (PC :type Player%20Controller%20Object%20Reference) (visibilities :type Array%20of%20Booleans) (items :type Array%20of%20Item%20Structur%20Structures))
  ;[1 0.1453 0.1354 1 142] Add this to your Playercontroller
  ;;[1 1 1] Update the ChestUI if this player is near to the chest and if the call for the update is not from this player
  (if (and (== chest (Variables|Default|GetcurrentChestRef)) (!= PC self))
    (bind _asbp_my_hud (Utilities|Casting|CastToBP_MyHUD (HUD|GetHUD)))
    (Default|UpateOwnChestUI (Variables|/Game/Asset/UI/Inventory/WB_Inventory.WB_Inventory_C|GetChestUI (Variables|/Game/Asset/UI/Inventory/WB_UI.WB_UI_C|GetInventory (Variables|/Game/AdvancedInventory/Blueprints/BP_MyHUD.BP_MyHUD_C|GetUI_Ref _asbp_my_hud))) (Variables|Default|GetcurrentChestRef) visibilities items)))

(event Custom|%28Un%29EquipItemFromEquipSlot
  (params (EquipSlot :type Object%20Object%20Reference) (fromEquipSlot? :type Boolean) (itemRefOnlyForEquipSlot :type WB%20Item%20Object%20Reference))
  ;[1 0.1453 0.1354 1 142] Add this to your Playercontroller
  ;;[1 1 1 1 30] Equip and Unequip items
  (if fromEquipSlot?
    _
    (else
      (bind _aswb_equip_slot (Utilities|Casting|CastToWB_EquipSlot EquipSlot))))
  (Class|BPInventoryInterface|EquipBody(Message) (Game|GetPlayerCharacter 0) (.StaticMesh (Utilities|Struct|BreakItem_Structur (Variables|/Game/Asset/UI/Inventory/WB_Item.WB_Item_C|GetItemData (select fromEquipSlot? itemRefOnlyForEquipSlot (Variables|/Game/Asset/UI/Inventory/WB_EquipSlot.WB_EquipSlot_C|GetItemWB _aswb_equip_slot))))) (.category (Utilities|Struct|BreakItem_Structur (Variables|/Game/Asset/UI/Inventory/WB_Item.WB_Item_C|GetItemData (select fromEquipSlot? itemRefOnlyForEquipSlot (Variables|/Game/Asset/UI/Inventory/WB_EquipSlot.WB_EquipSlot_C|GetItemWB _aswb_equip_slot))))) (Widget|IsVisible (select fromEquipSlot? itemRefOnlyForEquipSlot (Variables|/Game/Asset/UI/Inventory/WB_EquipSlot.WB_EquipSlot_C|GetItemWB _aswb_equip_slot))) (.relativeTransformInHand (Utilities|Struct|BreakItem_Structur (Variables|/Game/Asset/UI/Inventory/WB_Item.WB_Item_C|GetItemData (select fromEquipSlot? itemRefOnlyForEquipSlot (Variables|/Game/Asset/UI/Inventory/WB_EquipSlot.WB_EquipSlot_C|GetItemWB _aswb_equip_slot))))) (.relativeTransformEquiped (Utilities|Struct|BreakItem_Structur (Variables|/Game/Asset/UI/Inventory/WB_Item.WB_Item_C|GetItemData (select fromEquipSlot? itemRefOnlyForEquipSlot (Variables|/Game/Asset/UI/Inventory/WB_EquipSlot.WB_EquipSlot_C|GetItemWB _aswb_equip_slot)))))))

(event Custom|ToggleInventoryVisibility
  (bind (_sizex _sizey) (HUD|GetViewportSize))
  ;[1 0.1453 0.1354 1 142] Add this to your Playercontroller
  ;;[1 1 1] Toggle inventory visibility, input mode and mouse cursor visibility
  (if (Variables|Default|GetInventoryOn?)
    (Input|SetInputModeGameOnly self false)
    (Variables|Default|SetbShowMouseCursor false)
    (bind _asbp_my_hud (Utilities|Casting|CastToBP_MyHUD (HUD|GetHUD)))
    (Default|ShowHideInventory (Variables|/Game/Asset/UI/Inventory/WB_UI.WB_UI_C|GetInventory (Variables|/Game/AdvancedInventory/Blueprints/BP_MyHUD.BP_MyHUD_C|GetUI_Ref _asbp_my_hud)) false)
    (Variables|Default|SetInventoryOn? false)
    (Widget|SetVisibility (Variables|/Game/Asset/UI/Inventory/WB_Inventory.WB_Inventory_C|GetRightClickMenuRef (Variables|/Game/Asset/UI/Inventory/WB_UI.WB_UI_C|GetInventory (Variables|/Game/AdvancedInventory/Blueprints/BP_MyHUD.BP_MyHUD_C|GetUI_Ref _asbp_my_hud))) "Collapsed")
    (else
      (Input|SetInputModeGameandUI self 0 "DoNotLock" false false)
      (Variables|Default|SetbShowMouseCursor true)
      (bind _asbp_my_hud_2 (Utilities|Casting|CastToBP_MyHUD (HUD|GetHUD)))
      (Default|ShowHideInventory (Variables|/Game/Asset/UI/Inventory/WB_UI.WB_UI_C|GetInventory (Variables|/Game/AdvancedInventory/Blueprints/BP_MyHUD.BP_MyHUD_C|GetUI_Ref _asbp_my_hud_2)) true)
      (Variables|Default|SetInventoryOn? true)))
  (Class|PlayerController|SetMouseLocation (/ _sizex 2) (/ _sizey 2)))

(event Custom|UpdateGroundItemList
  ;[1 0.1453 0.1354 1 142] Add this to your Playercontroller
  ;;[1 1 1 1 30] For the GroundItemList
  ;;;[1 1 1] Update the GroundItemList
  (Default|UpdateGroundItemList (Variables|Default|GetInventoryComponentRef)))

(event Custom|DropEvent
  (params (ItemData :type Item%20Structur%20Structure))
  ;[1 0.1453 0.1354 1 142] Add this to your Playercontroller
  ;;[1 1 1 1 30] Event for dropping an item
  (Default|DropEvent (Variables|Default|GetInventoryComponentRef) ItemData))

(event Custom|getNewSlotDataAndCallUpdateForCharcater
  ;[1 0.1453 0.1354 1 142] Add this to your Playercontroller
  ;;[1 1 1 1 30] Equip and Unequip items
  (bind _asbp_my_hud (Utilities|Casting|CastToBP_MyHUD (HUD|GetHUD)))
  (bind _aswb_slot (Utilities|Casting|CastToWB_Slot (Class|PanelWidget|GetChildat (Variables|/Game/Asset/UI/Inventory/WB_Inventory.WB_Inventory_C|GetHotbar (Variables|/Game/Asset/UI/Inventory/WB_UI.WB_UI_C|GetInventory (Variables|/Game/AdvancedInventory/Blueprints/BP_MyHUD.BP_MyHUD_C|GetUI_Ref _asbp_my_hud))) (Variables|Default|GetcurrentSlot))))
  (Class|BPInventoryInterface|EquipRightHand(Message) (Game|GetPlayerCharacter 0) (.StaticMesh (Utilities|Struct|BreakItem_Structur (Variables|/Game/Asset/UI/Inventory/WB_Item.WB_Item_C|GetItemData (Variables|/Game/Asset/UI/Inventory/WB_Slot.WB_Slot_C|GetItemWB _aswb_slot)))) (.category (Utilities|Struct|BreakItem_Structur (Variables|/Game/Asset/UI/Inventory/WB_Item.WB_Item_C|GetItemData (Variables|/Game/Asset/UI/Inventory/WB_Slot.WB_Slot_C|GetItemWB _aswb_slot)))) (Widget|IsVisible (Variables|/Game/Asset/UI/Inventory/WB_Slot.WB_Slot_C|GetItemWB _aswb_slot)) (.relativeTransformInHand (Utilities|Struct|BreakItem_Structur (Variables|/Game/Asset/UI/Inventory/WB_Item.WB_Item_C|GetItemData (Variables|/Game/Asset/UI/Inventory/WB_Slot.WB_Slot_C|GetItemWB _aswb_slot)))) (.relativeTransformEquiped (Utilities|Struct|BreakItem_Structur (Variables|/Game/Asset/UI/Inventory/WB_Item.WB_Item_C|GetItemData (Variables|/Game/Asset/UI/Inventory/WB_Slot.WB_Slot_C|GetItemWB _aswb_slot))))))

(event Custom|ChangeSlot
  (params (mouseWheelUp? :type Boolean) (mouseWheelDown? :type Boolean) (keyboardNumber :type Integer))
  ;[1 0.1453 0.1354 1 142] Add this to your Playercontroller
  ;;[1 1 1 1 30] selection event for mouse wheel and keyboard input
  (bind _asbp_my_hud (Utilities|Casting|CastToBP_MyHUD (HUD|GetHUD)))
  (if (or mouseWheelUp? mouseWheelDown?)
    (if (Variables|Default|GetInventoryOn?)
      (Utilities|FlowControl|Delay 0.02)
      (if (not (Variables|/Game/Asset/UI/Inventory/WB_Inventory.WB_Inventory_C|GetblockSlotScrolling (Variables|/Game/Asset/UI/Inventory/WB_UI.WB_UI_C|GetInventory (Variables|/Game/AdvancedInventory/Blueprints/BP_MyHUD.BP_MyHUD_C|GetUI_Ref _asbp_my_hud))))
        (bind _aswb_slot (Utilities|Casting|CastToWB_Slot (Class|PanelWidget|GetChildat (Variables|/Game/Asset/UI/Inventory/WB_Inventory.WB_Inventory_C|GetHotbar (Variables|/Game/Asset/UI/Inventory/WB_UI.WB_UI_C|GetInventory (Variables|/Game/AdvancedInventory/Blueprints/BP_MyHUD.BP_MyHUD_C|GetUI_Ref _asbp_my_hud))) (Variables|Default|GetcurrentSlot)) :!label _label))
        (Default|Select _aswb_slot false)
        (if mouseWheelDown?
          (Math|Integer|IncrementInt (Variables|Default|GetcurrentSlot)
            (:%20%20
              (if (> (Variables|Default|GetcurrentSlot) (- (Class|PanelWidget|GetChildrenCount (Variables|/Game/Asset/UI/Inventory/WB_Inventory.WB_Inventory_C|GetHotbar (Variables|/Game/Asset/UI/Inventory/WB_UI.WB_UI_C|GetInventory (Variables|/Game/AdvancedInventory/Blueprints/BP_MyHUD.BP_MyHUD_C|GetUI_Ref _asbp_my_hud)))) 1))
                (Variables|Default|SetcurrentSlot 0)
                (CallFunction|SelecttheNewSlotSlot)
                (else
                  (CallFunction|SelecttheNewSlotSlot)))))
          (else
            (Math|Integer|DecrementInt (Variables|Default|GetcurrentSlot)
              (:%20%20
                (if (< (Variables|Default|GetcurrentSlot) 0)
                  (Variables|Default|SetcurrentSlot (- (Class|PanelWidget|GetChildrenCount (Variables|/Game/Asset/UI/Inventory/WB_Inventory.WB_Inventory_C|GetHotbar (Variables|/Game/Asset/UI/Inventory/WB_UI.WB_UI_C|GetInventory (Variables|/Game/AdvancedInventory/Blueprints/BP_MyHUD.BP_MyHUD_C|GetUI_Ref _asbp_my_hud)))) 1))
                  (CallFunction|SelecttheNewSlotSlot)
                  (else
                    (CallFunction|SelecttheNewSlotSlot))))))))
      (else
        (goto _label)))
    (elif (and (!= (Variables|Default|GetcurrentSlot) keyboardNumber) (<= keyboardNumber (- (Class|PanelWidget|GetChildrenCount (Variables|/Game/Asset/UI/Inventory/WB_Inventory.WB_Inventory_C|GetHotbar (Variables|/Game/Asset/UI/Inventory/WB_UI.WB_UI_C|GetInventory (Variables|/Game/AdvancedInventory/Blueprints/BP_MyHUD.BP_MyHUD_C|GetUI_Ref _asbp_my_hud)))) 1)))
      (bind _aswb_slot_2 (Utilities|Casting|CastToWB_Slot (Class|PanelWidget|GetChildat (Variables|/Game/Asset/UI/Inventory/WB_Inventory.WB_Inventory_C|GetHotbar (Variables|/Game/Asset/UI/Inventory/WB_UI.WB_UI_C|GetInventory (Variables|/Game/AdvancedInventory/Blueprints/BP_MyHUD.BP_MyHUD_C|GetUI_Ref _asbp_my_hud))) (Variables|Default|GetcurrentSlot))))
      (Default|Select _aswb_slot_2 false)
      (Variables|Default|SetcurrentSlot keyboardNumber)
      (CallFunction|SelecttheNewSlotSlot))))

(event EventBeginPlay
  ;[1 0.1453 0.1354 1 142] Add this to your Playercontroller
  ;;[1 1 1] Event BeginPlay
  ;;;[1 1 1 1 30] Select First slot on event begin play and set CharacterRef
  (Utilities|FlowControl|Delay 0.2)
  (bind _asbp_my_hud (Utilities|Casting|CastToBP_MyHUD (HUD|GetHUD)))
  (bind _aswb_slot (Utilities|Casting|CastToWB_Slot (Class|PanelWidget|GetChildat (Variables|/Game/Asset/UI/Inventory/WB_Inventory.WB_Inventory_C|GetHotbar (Variables|/Game/Asset/UI/Inventory/WB_UI.WB_UI_C|GetInventory (Variables|/Game/AdvancedInventory/Blueprints/BP_MyHUD.BP_MyHUD_C|GetUI_Ref _asbp_my_hud))))))
  (Default|Select _aswb_slot true))

(event Input|KeyboardEvents|I
  (params (Key :type Key%20Structure :default "None"))
  ;[1 0.1453 0.1354 1 142] Add this to your Playercontroller
  ;;[1 1 1 1 30] Key for show and Hide the inventory
  ;;;[0 1 0.3284] example
  (:Pressed
    (CallFunction|ToggleInventoryVisibility)))

(event Input|KeyboardEvents|H
  (params (Key :type Key%20Structure :default "None"))
  ;[1 0.1453 0.1354 1 142] Add this to your Playercontroller
  ;;[0 1 0.3284] Only for testing the inventory - add certain items to the inventory [example]
  (:Pressed
    (bind _asbp_my_hud (Utilities|Casting|CastToBP_MyHUD (HUD|GetHUD)))
    ;;;[1 1 1 1 12] Amount can be bigger than the max. stack size -> add items to new slots
    (Default|AddItem (Variables|/Game/Asset/UI/Inventory/WB_UI.WB_UI_C|GetInventory (Variables|/Game/AdvancedInventory/Blueprints/BP_MyHUD.BP_MyHUD_C|GetUI_Ref _asbp_my_hud)) 1 10)))

(event Input|MouseEvents|MouseWheelUp
  (params (Key :type Key%20Structure :default "None"))
  ;[1 0.1453 0.1354 1 142] Add this to your Playercontroller
  ;;[1 1 1] Mouse input for weapon Hotbar
  (:Pressed
    (if (== (Variables|Default|GetcurrentSlot) 0)
      (CallFunction|ChangeSlot false false 1)
      (else
        (CallFunction|ChangeSlot false false)))))

(event Input|KeyboardEvents|P
  (params (Key :type Key%20Structure :default "None"))
  (bind _autopickupmoderadiusref (Variables|Default|GetAutoPickupModeRadiusRef))
  ;[1 0.1453 0.1354 1 142] Add this to your Playercontroller
  ;;[1 1 1] Auto Pickup Mode
  (:Pressed
    (bind _asbp_my_hud (Utilities|Casting|CastToBP_MyHUD (HUD|GetHUD)))
    (if (Variables|Default|GetAutoPickupItemsMode)
      (Variables|Default|SetAutoPickupItemsMode false)
      (Default|ToggleAutoPickupMode (Variables|/Game/Asset/UI/Inventory/WB_UI.WB_UI_C|GetInventory (Variables|/Game/AdvancedInventory/Blueprints/BP_MyHUD.BP_MyHUD_C|GetUI_Ref _asbp_my_hud)) false)
      (Collision|SetCollisionEnabled _autopickupmoderadiusref "NoCollision")
      (else
        (Variables|Default|SetAutoPickupItemsMode true)
        (Default|ToggleAutoPickupMode (Variables|/Game/Asset/UI/Inventory/WB_UI.WB_UI_C|GetInventory (Variables|/Game/AdvancedInventory/Blueprints/BP_MyHUD.BP_MyHUD_C|GetUI_Ref _asbp_my_hud)) true)
        (Collision|SetCollisionEnabled _autopickupmoderadiusref "QueryOnly")))))

(event Input|KeyboardEvents|L
  (params (Key :type Key%20Structure :default "None"))
  ;[1 0.1453 0.1354 1 142] Add this to your Playercontroller
  ;;[1 1 1] Save & Load Slots
  (:Pressed
    (Utilities|FlowControl|Delay 0.2)
    (CallFunction|LoadAllInventorySlots)
    (CallFunction|GetNewSlotDataandCallUpdateforCharcater)))

(event Input|KeyboardEvents|O
  (params (Key :type Key%20Structure :default "None"))
  ;[1 0.1453 0.1354 1 142] Add this to your Playercontroller
  ;;[1 1 1] Save & Load Slots
  (:Pressed
    (CallFunction|SaveAllInventorySlots)))

(event Input|MouseEvents|RightMouseButton
  (params (Key :type Key%20Structure :default "None"))
  ;[1 0.1453 0.1354 1 142] Add this to your Playercontroller
  ;;[1 1 1] Equip armor on RightClick (when inventory is closed)
  (:Pressed
    (if (not (Variables|Default|GetInventoryOn?))
      (bind _asbp_my_hud (Utilities|Casting|CastToBP_MyHUD (HUD|GetHUD)))
      (bind _aswb_slot (Utilities|Casting|CastToWB_Slot (Class|PanelWidget|GetChildat (Variables|/Game/Asset/UI/Inventory/WB_Inventory.WB_Inventory_C|GetHotbar (Variables|/Game/Asset/UI/Inventory/WB_UI.WB_UI_C|GetInventory (Variables|/Game/AdvancedInventory/Blueprints/BP_MyHUD.BP_MyHUD_C|GetUI_Ref _asbp_my_hud))) (Variables|Default|GetcurrentSlot))))
      (if (and (Widget|IsVisible (Variables|/Game/Asset/UI/Inventory/WB_Slot.WB_Slot_C|GetItemWB _aswb_slot)) (.itemForEquipSlot? (Utilities|Struct|BreakItem_Structur (Variables|/Game/Asset/UI/Inventory/WB_Item.WB_Item_C|GetItemData (Variables|/Game/Asset/UI/Inventory/WB_Slot.WB_Slot_C|GetItemWB _aswb_slot)))))
        (bind _array_element (Utilities|Array|ForEachLoopwithBreak (Class|PanelWidget|GetAllChildren (Variables|/Game/Asset/UI/Inventory/WB_EquipInventory.WB_EquipInventory_C|GetEquipSlots (Variables|/Game/Asset/UI/Inventory/WB_Inventory.WB_Inventory_C|GetmanEq (Variables|/Game/Asset/UI/Inventory/WB_UI.WB_UI_C|GetInventory (Variables|/Game/AdvancedInventory/Blueprints/BP_MyHUD.BP_MyHUD_C|GetUI_Ref _asbp_my_hud))))) :!label _label)
          (:LoopBody
            (bind _aswb_equip_slot (Utilities|Casting|CastToWB_EquipSlot _array_element))
            (if (== (Variables|/Game/Asset/UI/Inventory/WB_EquipSlot.WB_EquipSlot_C|Getcategory _aswb_equip_slot) (.category (Utilities|Struct|BreakItem_Structur (Variables|/Game/Asset/UI/Inventory/WB_Item.WB_Item_C|GetItemData (Variables|/Game/Asset/UI/Inventory/WB_Slot.WB_Slot_C|GetItemWB _aswb_slot)))))
              (if (Widget|IsVisible (Variables|/Game/Asset/UI/Inventory/WB_EquipSlot.WB_EquipSlot_C|GetItemWB _aswb_equip_slot))
                (Variables|Default|SetSaveFix (Variables|/Game/Asset/UI/Inventory/WB_Item.WB_Item_C|GetItemData (Variables|/Game/Asset/UI/Inventory/WB_Slot.WB_Slot_C|GetItemWB _aswb_slot)))
                (Default|Update (Variables|/Game/Asset/UI/Inventory/WB_Slot.WB_Slot_C|GetItemWB _aswb_slot) (Variables|/Game/Asset/UI/Inventory/WB_Item.WB_Item_C|GetItemData (Variables|/Game/Asset/UI/Inventory/WB_EquipSlot.WB_EquipSlot_C|GetItemWB _aswb_equip_slot)))
                (Default|Update (Variables|/Game/Asset/UI/Inventory/WB_EquipSlot.WB_EquipSlot_C|GetItemWB _aswb_equip_slot) (Variables|Default|GetSaveFix))
                (else
                  (Default|HideShowItem (Variables|/Game/Asset/UI/Inventory/WB_EquipSlot.WB_EquipSlot_C|GetItemWB _aswb_equip_slot) true)
                  (Default|Activate _aswb_equip_slot true)
                  (Default|Update (Variables|/Game/Asset/UI/Inventory/WB_EquipSlot.WB_EquipSlot_C|GetItemWB _aswb_equip_slot) (Variables|/Game/Asset/UI/Inventory/WB_Item.WB_Item_C|GetItemData (Variables|/Game/Asset/UI/Inventory/WB_Slot.WB_Slot_C|GetItemWB _aswb_slot)))
                  (Default|HideShowItem (Variables|/Game/Asset/UI/Inventory/WB_Slot.WB_Slot_C|GetItemWB _aswb_slot) false)))
              (CallFunction|(Un)EquipItemfromEquipSlot _aswb_equip_slot false)
              (goto _label Break)))
          (:Completed
            (CallFunction|GetNewSlotDataandCallUpdateforCharcater)))))))

(event Input|MouseEvents|MiddleMouseButton
  (params (Key :type Key%20Structure :default "None"))
  ;[1 0.1453 0.1354 1 142] Add this to your Playercontroller
  ;;[1 1 1] Mouse input for weapon Hotbar
  (:Pressed
    (if (== (Variables|Default|GetcurrentSlot) 0)
      (CallFunction|ChangeSlot false false 1)
      (else
        (CallFunction|ChangeSlot false false)))))

(event Input|KeyboardEvents|F
  (params (Key :type Key%20Structure :default "None"))
  ;[1 0.1453 0.1354 1 142] Add this to your Playercontroller
  ;;[1 1 1 1 30] Key for show and Hide the inventory
  ;;;[0 1 0.3284] example
  (:Pressed
    (CallFunction|ToggleInventoryVisibility)))

(event Input|KeyboardEvents|G
  (params (Key :type Key%20Structure :default "None"))
  ;[1 0.1453 0.1354 1 142] Add this to your Playercontroller
  ;;[0 1 0.3284] Only for testing the inventory - add certain items to the inventory [example]
  (:Pressed
    (bind _asbp_my_hud (Utilities|Casting|CastToBP_MyHUD (HUD|GetHUD)))
    ;;;[1 1 1 1 12] Amount can be bigger than the max. stack size -> add items to new slots
    (Default|AddItem (Variables|/Game/Asset/UI/Inventory/WB_UI.WB_UI_C|GetInventory (Variables|/Game/AdvancedInventory/Blueprints/BP_MyHUD.BP_MyHUD_C|GetUI_Ref _asbp_my_hud)) 0 10)))

(event Input|MouseEvents|MouseWheelDown
  (params (Key :type Key%20Structure :default "None"))
  ;[1 0.1453 0.1354 1 142] Add this to your Playercontroller
  ;;[1 1 1] Mouse input for weapon Hotbar
  (:Pressed
    (if (== (Variables|Default|GetcurrentSlot) 0)
      (CallFunction|ChangeSlot false false 1)
      (else
        (CallFunction|ChangeSlot false false)))))

(event Input|KeyboardEvents|1
  (params (Key :type Key%20Structure :default "None"))
  ;[1 0.1453 0.1354 1 142] Add this to your Playercontroller
  ;;[1 1 1] Keyboard input for item use
  (:Pressed
    (CallFunction|ChangeSlot false false)))

(event Input|KeyboardEvents|2
  (params (Key :type Key%20Structure :default "None"))
  ;[1 0.1453 0.1354 1 142] Add this to your Playercontroller
  ;;[1 1 1] Keyboard input for item use
  (:Pressed
    (CallFunction|ChangeSlot false false 1)))

(event Input|KeyboardEvents|3
  (params (Key :type Key%20Structure :default "None"))
  ;[1 0.1453 0.1354 1 142] Add this to your Playercontroller
  ;;[1 1 1] Keyboard input for item use
  (:Pressed
    (CallFunction|ChangeSlot false false 2)))

(event Input|KeyboardEvents|Z
  (params (Key :type Key%20Structure :default "None"))
  ;[1 0.1453 0.1354 1 142] Add this to your Playercontroller
  (:Pressed
    (bind _asbp_my_hud (Utilities|Casting|CastToBP_MyHUD (HUD|GetHUD)))
    (Default|AddItem (Variables|/Game/Asset/UI/Inventory/WB_UI.WB_UI_C|GetInventory (Variables|/Game/AdvancedInventory/Blueprints/BP_MyHUD.BP_MyHUD_C|GetUI_Ref _asbp_my_hud)) 8 1)))

(event Input|KeyboardEvents|J
  (params (Key :type Key%20Structure :default "None"))
  ;[1 0.1453 0.1354 1 142] Add this to your Playercontroller
  ;;[0 1 0.3284] Only for testing the inventory - add certain items to the inventory [example]
  (:Pressed
    (bind _asbp_my_hud (Utilities|Casting|CastToBP_MyHUD (HUD|GetHUD)))
    ;;;[1 1 1 1 12] Amount can be bigger than the max. stack size -> add items to new slots
    (Default|AddItem (Variables|/Game/Asset/UI/Inventory/WB_UI.WB_UI_C|GetInventory (Variables|/Game/AdvancedInventory/Blueprints/BP_MyHUD.BP_MyHUD_C|GetUI_Ref _asbp_my_hud)) 2 10)))

(fn ConstructionScript)

(fn SaveAllInventorySlots
  (bind _asbp_my_hud (Utilities|Casting|CastToBP_MyHUD (HUD|GetHUD)))
  (for _array_element (Variables|/Game/Asset/UI/Inventory/WB_Inventory.WB_Inventory_C|GetAllInventoryBars (Variables|/Game/Asset/UI/Inventory/WB_UI.WB_UI_C|GetInventory (Variables|/Game/AdvancedInventory/Blueprints/BP_MyHUD.BP_MyHUD_C|GetUI_Ref _asbp_my_hud)))
    (bind _ashorizontal_box (Utilities|Casting|CastToHorizontalBox _array_element))
    (for _array_element_2 (Class|PanelWidget|GetAllChildren _ashorizontal_box)
      (bind _aswb_slot (Utilities|Casting|CastToWB_Slot _array_element_2))
      (Utilities|Array|Add (LocalVariables|GetAllSlotVisibilities) (Widget|IsVisible (Variables|/Game/Asset/UI/Inventory/WB_Slot.WB_Slot_C|GetItemWB _aswb_slot)))
      (if (Widget|IsVisible (Variables|/Game/Asset/UI/Inventory/WB_Slot.WB_Slot_C|GetItemWB _aswb_slot))
        (Utilities|Array|Add (LocalVariables|GetAllSlotDatas) (Variables|/Game/Asset/UI/Inventory/WB_Item.WB_Item_C|GetItemData (Variables|/Game/Asset/UI/Inventory/WB_Slot.WB_Slot_C|GetItemWB _aswb_slot)))
        (else
          (Utilities|Array|Add :TargetArray (LocalVariables|GetAllSlotDatas))))))
  (for _array_element_3 (Class|PanelWidget|GetAllChildren (Variables|/Game/Asset/UI/Inventory/WB_EquipInventory.WB_EquipInventory_C|GetEquipSlots (Variables|/Game/Asset/UI/Inventory/WB_Inventory.WB_Inventory_C|GetmanEq (Variables|/Game/Asset/UI/Inventory/WB_UI.WB_UI_C|GetInventory (Variables|/Game/AdvancedInventory/Blueprints/BP_MyHUD.BP_MyHUD_C|GetUI_Ref _asbp_my_hud)))))
    (bind _aswb_equip_slot (Utilities|Casting|CastToWB_EquipSlot _array_element_3))
    (Utilities|Array|Add (LocalVariables|GetAllEquipSlotVisibilities) (Widget|IsVisible (Variables|/Game/Asset/UI/Inventory/WB_EquipSlot.WB_EquipSlot_C|GetItemWB _aswb_equip_slot)))
    (if (Widget|IsVisible (Variables|/Game/Asset/UI/Inventory/WB_EquipSlot.WB_EquipSlot_C|GetItemWB _aswb_equip_slot))
      (Utilities|Array|Add (LocalVariables|GetAllEquipSlotDatas) (Variables|/Game/Asset/UI/Inventory/WB_Item.WB_Item_C|GetItemData (Variables|/Game/Asset/UI/Inventory/WB_EquipSlot.WB_EquipSlot_C|GetItemWB _aswb_equip_slot)))
      (else
        (Utilities|Array|Add :TargetArray (LocalVariables|GetAllEquipSlotDatas)))))
  (bind _returnvalue (SaveGame|CreateSaveGameObject "/Game/AdvancedInventory/Blueprints/BP_InventorySaveObject.BP_InventorySaveObject_C"))
  (bind _output_get (Variables|Default|SetInventorySave _returnvalue))
  (Variables|/Game/AdvancedInventory/Blueprints/BP_InventorySaveObject.BP_InventorySaveObject_C|SetAllSlotVisibilitiesSave _output_get (LocalVariables|GetAllSlotVisibilities))
  (Variables|/Game/AdvancedInventory/Blueprints/BP_InventorySaveObject.BP_InventorySaveObject_C|SetAllSlotDatasSave _output_get (LocalVariables|GetAllSlotDatas))
  (Variables|/Game/AdvancedInventory/Blueprints/BP_InventorySaveObject.BP_InventorySaveObject_C|SetAllEquipSlotVisibilitiesSave _output_get (LocalVariables|GetAllEquipSlotVisibilities))
  (Variables|/Game/AdvancedInventory/Blueprints/BP_InventorySaveObject.BP_InventorySaveObject_C|SetAllEquipSlotDatasSave _output_get (LocalVariables|GetAllEquipSlotDatas))
  (SaveGame|SaveGametoSlot _output_get (Variables|Default|GetSaveSlotName)))

(fn LoadAllInventorySlots
  (bind _returnvalue (SaveGame|DoesSaveGameExist (Variables|Default|GetSaveSlotName)))
  (if _returnvalue
    (bind _returnvalue_2 (SaveGame|LoadGamefromSlot (Variables|Default|GetSaveSlotName)))
    (bind _asbp_inventory_save_object (Utilities|Casting|CastToBP_InventorySaveObject _returnvalue_2))
    (LocalVariables|SetAllSlotVisibilities (Variables|/Game/AdvancedInventory/Blueprints/BP_InventorySaveObject.BP_InventorySaveObject_C|GetAllSlotVisibilitiesSave _asbp_inventory_save_object))
    (LocalVariables|SetAllSlotDatas (Variables|/Game/AdvancedInventory/Blueprints/BP_InventorySaveObject.BP_InventorySaveObject_C|GetAllSlotDatasSave _asbp_inventory_save_object))
    (LocalVariables|SetAllEquipSlotVisibilities (Variables|/Game/AdvancedInventory/Blueprints/BP_InventorySaveObject.BP_InventorySaveObject_C|GetAllEquipSlotVisibilitiesSave _asbp_inventory_save_object))
    (LocalVariables|SetAllEquipSlotDatas (Variables|/Game/AdvancedInventory/Blueprints/BP_InventorySaveObject.BP_InventorySaveObject_C|GetAllEquipSlotDatasSave _asbp_inventory_save_object))
    (bind _asbp_my_hud (Utilities|Casting|CastToBP_MyHUD (HUD|GetHUD)))
    (for (_array_element _array_index) (Variables|/Game/Asset/UI/Inventory/WB_Inventory.WB_Inventory_C|GetAllInventoryBars (Variables|/Game/Asset/UI/Inventory/WB_UI.WB_UI_C|GetInventory (Variables|/Game/AdvancedInventory/Blueprints/BP_MyHUD.BP_MyHUD_C|GetUI_Ref _asbp_my_hud)))
      (bind _ashorizontal_box (Utilities|Casting|CastToHorizontalBox _array_element))
      (for (_array_element_2 _array_index_2) (Class|PanelWidget|GetAllChildren _ashorizontal_box)
        (bind _aswb_slot (Utilities|Casting|CastToWB_Slot _array_element_2))
        (if (Utilities|Array|Get(acopy) (LocalVariables|GetAllSlotVisibilities) (+ _array_index_2 (* (Utilities|Array|Length (Class|PanelWidget|GetAllChildren _ashorizontal_box)) _array_index)))
          (Default|HideShowItem (Variables|/Game/Asset/UI/Inventory/WB_Slot.WB_Slot_C|GetItemWB _aswb_slot) true)
          (Default|Update (Variables|/Game/Asset/UI/Inventory/WB_Slot.WB_Slot_C|GetItemWB _aswb_slot) (Utilities|Array|Get(acopy) (LocalVariables|GetAllSlotDatas) (+ _array_index_2 (* (Utilities|Array|Length (Class|PanelWidget|GetAllChildren _ashorizontal_box)) _array_index))))
          (else
            (Default|HideShowItem (Variables|/Game/Asset/UI/Inventory/WB_Slot.WB_Slot_C|GetItemWB _aswb_slot) false)))))
    (for (_array_element_3 _array_index_3) (Class|PanelWidget|GetAllChildren (Variables|/Game/Asset/UI/Inventory/WB_EquipInventory.WB_EquipInventory_C|GetEquipSlots (Variables|/Game/Asset/UI/Inventory/WB_Inventory.WB_Inventory_C|GetmanEq (Variables|/Game/Asset/UI/Inventory/WB_UI.WB_UI_C|GetInventory (Variables|/Game/AdvancedInventory/Blueprints/BP_MyHUD.BP_MyHUD_C|GetUI_Ref _asbp_my_hud)))))
      (bind _aswb_equip_slot (Utilities|Casting|CastToWB_EquipSlot _array_element_3))
      (Default|HideShowItem (Variables|/Game/Asset/UI/Inventory/WB_EquipSlot.WB_EquipSlot_C|GetItemWB _aswb_equip_slot) (Utilities|Array|Get(acopy) (LocalVariables|GetAllEquipSlotVisibilities) _array_index_3))
      (if (Utilities|Array|Get(acopy) (LocalVariables|GetAllEquipSlotVisibilities) _array_index_3)
        (Default|Update (Variables|/Game/Asset/UI/Inventory/WB_EquipSlot.WB_EquipSlot_C|GetItemWB _aswb_equip_slot) (Utilities|Array|Get(acopy) (LocalVariables|GetAllEquipSlotDatas) _array_index_3))
        (Default|Activate _aswb_equip_slot true)
        (CallFunction|(Un)EquipItemfromEquipSlot _aswb_equip_slot false (Variables|/Game/Asset/UI/Inventory/WB_EquipSlot.WB_EquipSlot_C|GetItemWB _aswb_equip_slot))))))

(fn GetGM
  (bind _asbp_inventory_game_mode (Utilities|Casting|CastToBP_InventoryGameMode (Game|GetGameMode)))
  (return _asbp_inventory_game_mode))