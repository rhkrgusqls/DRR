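; Warrior goblin stage monster Blueprint whose graph implements the DropItem event for loot.
; When player pawn 0 has authority, it looks up a random DataNum row name in ItemTable; RandomInteger on LastIndex never selects the final entry.
; A found row spawns an item actor above the goblin, facing its yaw, with the row data, a fixed speed and a pitch-derived vertical velocity.
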(event EventDropItem
  (bind _returnvalue (Transformation|GetActorLocation))
  (bind _returnvalue_2 (Transformation|GetActorRotation))
  (bind _datanum (Variables|Default|GetDataNum))
  (bind (_x _y _z) (Math|Vector|BreakVector _returnvalue))
  (if (Ability|HasAuthority (Game|Player|GetPlayerPawn 0))
    (Variables|Default|SetItemData "")
    (bind _returnvalue_3 (Utilities|GetDataTableRow (Variables|Default|GetItemTable) (Utilities|Array|Get(acopy) _datanum (Math|Random|RandomInteger (Utilities|Array|LastIndex _datanum))))
      (:then
        (Variables|Default|SetItemData _returnvalue_3)
        (Game|SpawnActorfromClass "/Game/AdvancedInventory/Blueprints/BP_DropItemActor_Master.BP_DropItemActor_Master_C" (Math|Transform|MakeTransform (Math|Vector|MakeVector _x _y (+ 4e+01 _z)) (Math|Rotator|MakeRotator 0.0 0.0 (.Yaw (Math|Rotator|BreakRotator _returnvalue_2)))) "Undefined" "OverrideRootScale" 0 3.0 (Variables|Default|GetItemData) (* (.Pitch (Math|Rotator|BreakRotator _returnvalue_2)) 12.0) 0.0 0)))))

(fn ConstructionScript)