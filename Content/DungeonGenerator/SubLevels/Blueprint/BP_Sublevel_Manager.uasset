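; Manager actor for a dungeon generator sublevel, streaming one named room in as a level instance at a given transform under a unique ID.
; On BeginPlay the authority loads it, polls on a timer until loaded, then fires LevelLoaded, or LevelError if invalid.
; Setting the replicated LoadLevel flag lets clients load their own copy through its RepNotify.
; UnloadLevel unloads by ID and clears both state flags.
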(event Custom|UnloadLevel
  (Variables|Default|SetLoadLevel false)
  (Utilities|UnloadLevel (Variables|Default|GetUniqueID))
  (Variables|Default|SetLevelActive false))

(event EventBeginPlay
  (bind _transform (Variables|Default|GetTransform))
  (Networking|SwitchHasAuthority
    (:Authority
      (bind _returnvalue (Class|LevelStreamingDynamic|LoadLevelInstance (Utilities|String|ToString(Name) (Variables|Default|GetName)) (.location _transform) (.rotation _transform) (Variables|Default|GetUniqueID) 0 false))
      (Variables|/Script/Engine.LevelStreaming|SetbShouldBeLoaded _returnvalue true)
      (Variables|/Script/Engine.LevelStreaming|SetbShouldBeVisible _returnvalue true)
      (if (Utilities|IsValid _returnvalue)
        (if (Class|LevelStreaming|IsLevelLoaded _returnvalue) :!label _label
          (Variables|Default|SetLevelActive true)
          (Variables|Default|SetLoadLevel true)
          (Default|CallLevelLoaded)
          (else
            (Utilities|FlowControl|Delay (Variables|Default|GetLoadTimer))
            (goto _label)))
        (else
          (Development|PrintString (Utilities|String|ToString(Text) (Utilities|Text|FormatText "Invalid. Cannot find Room \"{Room}\" in the list of sublevels" (Variables|Default|GetName))) true true "(R=1.000000,G=0.000000,B=0.000000,A=1.000000)" 1e+01)
          (Default|CallLevelError))))))

(fn ConstructionScript)

(fn OnRepLoadLevel
  (bind _transform (Variables|Default|GetTransform))
  (if (Variables|Default|GetLoadLevel)
    (if (not (Variables|Default|GetLevelActive))
      (bind _returnvalue (Class|LevelStreamingDynamic|LoadLevelInstance (Utilities|String|ToString(Name) (Variables|Default|GetName)) (.location _transform) (.rotation _transform) (Variables|Default|GetUniqueID) 0 false))
      (Variables|/Script/Engine.LevelStreaming|SetbShouldBeLoaded _returnvalue true)
      (Variables|/Script/Engine.LevelStreaming|SetbShouldBeVisible _returnvalue true)
      (Variables|Default|SetLevelActive true))))