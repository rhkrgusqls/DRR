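; BP_Door_Demo is a demo door for the dungeon generator map that swings open on overlap with its Box component and closes when the overlap ends.
; Each event runs a delayed loop that rotates Door in small fixed increments, with the DoorRot counter limiting travel to a quarter turn.
; Two opposing boolean flags stop the other loop, so the door can reverse mid-swing without using Tick or a Timeline.
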(event OnComponentBeginOverlap(Box)
  (params (OverlappedComponent :type Primitive%20Component%20Object%20Reference) (OtherActor :type Actor%20Object%20Reference) (OtherComp :type Primitive%20Component%20Object%20Reference) (OtherBodyIndex :type Integer) (bFromSweep :type Boolean) (SweepResult :type Hit%20Result%20Structure%20%28by%20ref%29))
  (Variables|Default|SetNewVar_0 true)
  (Variables|Default|SetNewVar false)
  (if (and (not (== (Variables|Default|GetDoorRot) 30)) (Variables|Default|GetNewVar_0)) :!label _label
    (Utilities|FlowControl|Delay 0.05)
    (Transformation|AddRelativeRotation (Variables|Default|GetDoor) "0.000000,3.000000,0.000000" false false)
    (Math|Integer|IncrementInt (Variables|Default|GetDoorRot)
      (:%20%20
        (goto _label)))))

(event OnComponentEndOverlap(Box)
  (params (OverlappedComponent :type Primitive%20Component%20Object%20Reference) (OtherActor :type Actor%20Object%20Reference) (OtherComp :type Primitive%20Component%20Object%20Reference) (OtherBodyIndex :type Integer))
  (Variables|Default|SetNewVar true)
  (Variables|Default|SetNewVar_0 false)
  (if (and (not (== (Variables|Default|GetDoorRot) 0)) (Variables|Default|GetNewVar)) :!label _label
    (Utilities|FlowControl|Delay 0.05)
    (Transformation|AddRelativeRotation (Variables|Default|GetDoor) "0.000000,-3.000000,0.000000" false false)
    (Math|Integer|DecrementInt (Variables|Default|GetDoorRot)
      (:%20%20
        (goto _label)))))

(event EventBeginPlay)

(event Collision|EventActorBeginOverlap
  (params (OtherActor :type Actor%20Object%20Reference)))

(event EventTick
  (params (DeltaSeconds :type Float%20%28single-precision%29)))

(fn ConstructionScript)